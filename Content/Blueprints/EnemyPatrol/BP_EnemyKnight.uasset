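; BP_EnemyKnight is an enemy knight that patrols by either random roaming or following target points, chosen by flags on BeginPlay.
; Roaming repeatedly moves to random reachable points nearby, pausing between moves and retrying on failure.
; Waypoint patrol loops through TargetPoints with a pause, wrapping upon reaching the last index, so that point is never visited; failed moves end it.
; Pawn sensing only prints "Spotted" for BP_FPAbility pawns.
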(event OnSeePawn(PawnSensing)
  (params (Pawn :type Pawn%20Object%20Reference))
  (Utilities|Casting|CastToBP_FPAbility Pawn)
  (Development|PrintString "Spotted"))

(event Custom|Roam%20Character
  ;[0.15 0.15 0.15 0.5] Roams Area
  (AI|AIMoveTo self (.RandomLocation (AI|Navigation|GetRandomReachablePointinRadius (Transformation|GetActorLocation) 1.5e+03 0 0)) 0 5.0 false
    (:OnSuccess
      _)
    (:OnFail
      _))
  (Utilities|FlowControl|Delay (Variables|KnightTask|GetHow%20Long%20is%20the%20Task?))
  (CallFunction|RoamCharacter))

(event Custom|Target%20Character
  ;[0.15 0.15 0.15 0.5] Target Character (Uses Target Points)
  (AI|AIMoveTo self "0, 0, 0" (Utilities|Array|Get(acopy) (Variables|Waypoints|GetTarget%20Points) (Variables|Waypoints|GetCurrent%20Waypoint)) 5.0 true
    (:OnSuccess
      (Math|Integer|IncrementInt (Variables|Waypoints|GetCurrent%20Waypoint)
        (:%20%20
          (Utilities|FlowControl|Delay (Variables|KnightTask|GetHow%20Long%20is%20the%20Task?))
          (if (== (Variables|Waypoints|GetCurrent%20Waypoint) (Variables|Waypoints|GetMax%20Waypoint))
            (Variables|Waypoints|SetCurrent%20Waypoint 0)
            (CallFunction|TargetCharacter)
            (else
              (CallFunction|TargetCharacter))))))))

(event EventBeginPlay
  ;[0.15 0.15 0.15 0.5] Guard Hierarchy
  (Utilities|FlowControl|Sequence
    (:then_0
      (if (Variables|KnightTask|GetbShouldKnightRoam?)
        (CallFunction|RoamCharacter)
        (elif (Variables|KnightTask|GetbShouldKnightTarget?)
          (CallFunction|TargetCharacter))))
    (:then_1
      ;[0.15 0.15 0.15 0.5] Sets Target Points To Max Waypoints
      (Variables|Waypoints|SetMax%20Waypoint (Utilities|Array|LastIndex (Variables|Waypoints|GetTarget%20Points))))))

(fn ConstructionScript)