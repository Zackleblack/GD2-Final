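; BP_BigDoorPotion is a double door that opens by itself once the player has gained the dash ability.
; It caches the AscendThroughTime game instance on BeginPlay and polls HasDashAbility every Tick.
; When the flag is set, a DoOnce triggers DoorOpens after a short delay.
; DoorOpens plays a creak sound using DoorRim's relative location and runs the Open timeline, swinging both leaves outward in yaw.
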(event Custom|Door%20Opens
  (Audio|PlaySoundatLocation "/Game/Free_Sounds_Pack/cue/Wood_and_Door_Creak_01_Cue.Wood_and_Door_Creak_01_Cue" (Variables|/Script/Engine.SceneComponent|GetRelativeLocation (Variables|Default|GetDoorRim)) "0, 0, 0" 1.0 1.0 0.0 0 0 0 0)
  (bind _left_door (Timeline|Open Play)
    (:Update
      (Transformation|SetRelativeRotation (Variables|Default|GetLeftDoor) (Math|Rotator|MakeRotator 0.0 0.0 (Math|Float|Lerp 0.0 -9e+01 _left_door)) false false)
      (Transformation|SetRelativeRotation (Variables|Default|GetRightDoor) (Math|Rotator|MakeRotator 0.0 0.0 (Math|Float|Lerp 0.0 98.0 _left_door)) false false))))

(event EventBeginPlay
  (bind _asascend_through_time (Utilities|Casting|CastToAscendThroughTime (Game|GetGameInstance)))
  (Variables|Default|SetGame%20Instance%20Ref _asascend_through_time))

(event EventTick
  (params (DeltaSeconds :type Float%20%28single-precision%29))
  (if (Variables|/Game/Blueprints/AscendThroughTime.AscendThroughTime_C|GetbHasDashAbility? (Variables|Default|GetGame%20Instance%20Ref))
    (Utilities|FlowControl|DoOnce false
      (:Completed
        (Utilities|FlowControl|Delay 2.0)
        (CallFunction|DoorOpens)))))

(fn ConstructionScript)