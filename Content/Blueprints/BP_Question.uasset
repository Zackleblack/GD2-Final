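; BP_Question is an interactable question mark actor that spins via a Timeline and shows a selected widget when used.
; Its Sphere overlap with the BP_FPAbility player sets Interactive and toggles the interact prompt from BP_FPAbilityHUD.
; Interact passes a DoOnce, then, if in range, swaps the prompt for the WidgetSelection widget for three seconds before resetting.
; An out-of-range Interact call consumes the DoOnce without resetting it.
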(event OnComponentBeginOverlap(Sphere)
  (params (OverlappedComponent :type Primitive%20Component%20Object%20Reference) (OtherActor :type Actor%20Object%20Reference) (OtherComp :type Primitive%20Component%20Object%20Reference) (OtherBodyIndex :type Integer) (bFromSweep :type Boolean) (SweepResult :type Hit%20Result%20Structure%20%28by%20ref%29))
  (Utilities|Casting|CastToBP_FPAbility OtherActor)
  (Variables|Default|SetbInteractive true)
  (UserInterface|Viewport|AddtoViewport (Variables|/Game/Blueprints/TimeTravel/BP_FPAbilityHUD.BP_FPAbilityHUD_C|GetInteract%20Widget%20Reference (Variables|Default|GetHUD%20Reference)) 0))

(event OnComponentEndOverlap(Sphere)
  (params (OverlappedComponent :type Primitive%20Component%20Object%20Reference) (OtherActor :type Actor%20Object%20Reference) (OtherComp :type Primitive%20Component%20Object%20Reference) (OtherBodyIndex :type Integer))
  (Utilities|Casting|CastToBP_FPAbility OtherActor)
  (Variables|Default|SetbInteractive false)
  (Widget|RemovefromParent (Variables|/Game/Blueprints/TimeTravel/BP_FPAbilityHUD.BP_FPAbilityHUD_C|GetInteract%20Widget%20Reference (Variables|Default|GetHUD%20Reference))))

(event Custom|Reset
  (Utilities|FlowControl|DoOnce false) ; enters at Reset
)

(event EventBeginPlay
  (Utilities|FlowControl|Sequence
    (:then_0
      (bind _newtrack_0 (Timeline|Timeline Play)
        (:Update
          (Transformation|SetRelativeRotation (Variables|Default|GetQuestion) (Math|Rotator|MakeRotator 0.0 0.0 (Math|Float|Lerp 0.0 3.6e+02 _newtrack_0)) false false))))
    (:then_1
      (bind _asbp_fpability (Utilities|Casting|CastToBP_FPAbility (Game|GetPlayerCharacter 0)))
      (Variables|Default|SetCharacter%20Reference _asbp_fpability))
    (:then_2
      (bind _returnvalue (Actor|GetActorOfClass "/Game/Blueprints/TimeTravel/BP_FPAbilityHUD.BP_FPAbilityHUD_C"))
      (Variables|Default|SetHUD%20Reference _returnvalue))))

(event EventInteract
  (Utilities|FlowControl|DoOnce false
    (:Completed
      (if (Variables|Default|GetbInteractive)
        (Widget|RemovefromParent (Variables|/Game/Blueprints/TimeTravel/BP_FPAbilityHUD.BP_FPAbilityHUD_C|GetInteract%20Widget%20Reference (Variables|Default|GetHUD%20Reference)))
        (bind _returnvalue (UserInterface|CreateWidget (Variables|Default|GetWidget%20Selection)))
        (bind _output_get (Variables|Default|SetWidget%20Used _returnvalue))
        (UserInterface|Viewport|AddtoViewport _output_get 0)
        (Utilities|FlowControl|Delay 3.0)
        (Widget|RemovefromParent (Variables|Default|GetWidget%20Used))
        (CallFunction|Reset)))))

(fn ConstructionScript)