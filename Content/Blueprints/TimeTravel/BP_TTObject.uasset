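; BP_TTObject is a time-travel prop that is solid in either the future or the present, set by ObjectFuture.
; Every Tick it reads AbilityOn from the player's BP_FPAbility and picks the tangible or intangible state.
; Tangible restores the mesh's material, collision and visible sparkles.
; Intangible applies a blue glitch material, disables collision, hides sparkles and calls audio play, repeating each frame while in that state.
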(event Custom|Set%20Time%20Objects%20Tangible
  (bind _staticmesh (Variables|Default|GetStaticMesh))
  (Rendering|Material|SetMaterial _staticmesh 0 (Rendering|Material|GetMaterial (Variables|Default|GetStatic%20Mesh%20Ref) 0))
  (Collision|SetCollisionEnabled _staticmesh "QueryAndPhysics")
  (Development|SetHiddeninGame (Variables|Default|GetSparkles) false false))

(event Custom|Set%20Time%20Objects%20Intangible
  (bind _staticmesh (Variables|Default|GetStaticMesh))
  (Rendering|Material|SetMaterial _staticmesh 0 "/Game/Blueprints/TimeTravel/MI_GlitchBlue.MI_GlitchBlue")
  (Collision|SetCollisionEnabled _staticmesh "NoCollision")
  (Development|SetHiddeninGame (Variables|Default|GetSparkles) true false)
  (Audio|Components|Audio|Play (Variables|Default|GetAudio) 0.0))

(event EventBeginPlay
  (Utilities|FlowControl|Sequence
    (:then_0
      (bind _asbp_fpability (Utilities|Casting|CastToBP_FPAbility (Game|GetPlayerCharacter 0)))
      (Variables|Default|SetPlayer%20Reference _asbp_fpability))
    (:then_1
      (Components|StaticMesh|SetStaticMesh (Variables|Default|GetStaticMesh) (Variables|Default|GetStatic%20Mesh%20Ref))
      (if (Variables|Default|GetbObjectFuture?)
        (CallFunction|SetTimeObjectsIntangible)
        (else
          (CallFunction|SetTimeObjectsTangible))))))

(event EventTick
  (params (DeltaSeconds :type Float%20%28single-precision%29))
  (bind _sparkles (Variables|Default|GetSparkles))
  (bind _staticmesh (Variables|Default|GetStaticMesh))
  (bind _staticmesh_2 (Variables|Default|GetStaticMesh))
  (if (Variables|/Game/Blueprints/TimeTravel/BP_FPAbility.BP_FPAbility_C|GetbAbilityOn? (Variables|Default|GetPlayer%20Reference))
    (if (Variables|Default|GetbObjectFuture?)
      (Rendering|Material|SetMaterial _staticmesh 0 (Rendering|Material|GetMaterial (Variables|Default|GetStatic%20Mesh%20Ref) 0) :!label _label)
      (Collision|SetCollisionEnabled _staticmesh "QueryAndPhysics")
      (Development|SetHiddeninGame _sparkles false false)
      (else
        (Rendering|Material|SetMaterial _staticmesh_2 0 "/Game/Blueprints/TimeTravel/MI_GlitchBlue.MI_GlitchBlue" :!label _label_2)
        (Collision|SetCollisionEnabled _staticmesh_2 "NoCollision")
        (Development|SetHiddeninGame _sparkles true false)
        (Audio|Components|Audio|Play (Variables|Default|GetAudio) 0.0)))
    (elif (Variables|Default|GetbObjectFuture?)
      (goto _label_2)
      (else
        (goto _label)))))

(fn ConstructionScript)