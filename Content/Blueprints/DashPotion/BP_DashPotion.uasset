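; A dash potion pickup that permanently sets the dash-unlocked flag on the BP_FPAbility player character.
; Two timelines spin and bob its static mesh, while a sphere overlap tracks whether the player is in range.
; An Interact event, when in range and not yet picked up, unlocks the dash, hides the mesh and disables its collision.
; It plays drink and burp sounds with delays, then destroys itself.
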(event OnComponentBeginOverlap(Sphere)
  (params (OverlappedComponent :type Primitive%20Component%20Object%20Reference) (OtherActor :type Actor%20Object%20Reference) (OtherComp :type Primitive%20Component%20Object%20Reference) (OtherBodyIndex :type Integer) (bFromSweep :type Boolean) (SweepResult :type Hit%20Result%20Structure%20%28by%20ref%29))
  ;[0 0.4678 0.5333 0.502] Is Player Within Range?
  (Utilities|Casting|CastToBP_FPAbility OtherActor)
  (Variables|Default|SetbInRange? true))

(event OnComponentEndOverlap(Sphere)
  (params (OverlappedComponent :type Primitive%20Component%20Object%20Reference) (OtherActor :type Actor%20Object%20Reference) (OtherComp :type Primitive%20Component%20Object%20Reference) (OtherBodyIndex :type Integer))
  ;[0 0.4678 0.5333 0.502] Is Player Within Range?
  (Utilities|Casting|CastToBP_FPAbility OtherActor)
  (Variables|Default|SetbInRange? false))

(event EventBeginPlay
  (bind _staticmesh (Variables|Default|GetStaticMesh))
  (bind _returnvalue (Transformation|GetRelativeTransform _staticmesh))
  ;[0 0.4678 0.5333 0.502] Bobing and Rotation
  (Utilities|FlowControl|Sequence
    (:then_0
      (bind _returnvalue_2 (Actor|GetActorOfClass "/Game/Blueprints/TimeTravel/BP_FPAbility.BP_FPAbility_C"))
      (Variables|Default|SetCharacter%20Reference _returnvalue_2))
    (:then_1
      (bind _loop (Timeline|Rotation Play)
        (:Update
          (Transformation|SetRelativeRotation _staticmesh (Math|Rotator|MakeRotator 0.0 0.0 (Math|Float|Lerp 0.0 3.6e+02 _loop)) false false))))
    (:then_2
      (bind _loop_2 (Timeline|Timeline Play)
        (:Update
          (Transformation|SetRelativeLocation _staticmesh (Math|Vector|MakeVector (.x (.location _returnvalue)) (.y (.location _returnvalue)) (Math|Float|Lerp 0.0 3e+01 _loop_2)) false false))))))

(event EventInteract
  (bind _staticmesh (Variables|Default|GetStaticMesh))
  ;[0 0.4678 0.5333 0.502] Interaction Pickup
  (if (Variables|Default|GetbInRange?)
    (if (not (Variables|Default|GetbPickedUp?))
      (Variables|/Game/Blueprints/TimeTravel/BP_FPAbility.BP_FPAbility_C|SetbDashAbilityUnlocked (Variables|Default|GetCharacter%20Reference) true)
      (Utilities|FlowControl|Sequence
        (:then_0
          (Audio|PlaySound2D "/Game/Blueprints/DashPotion/FreeSound_Glug.FreeSound_Glug" 1.0 1.0 0.0 0 0)
          (Utilities|FlowControl|Delay 1.0)
          (Audio|PlaySound2D "/Game/Blueprints/DashPotion/eritnhut1992-burp-20581.eritnhut1992-burp-20581" 0.5 1.0 0.0 0 0)
          (Utilities|FlowControl|Delay 2.5)
          (Actor|DestroyActor))
        (:then_1
          (Variables|Default|SetbPickedUp? true)
          (Development|SetHiddeninGame _staticmesh true false)
          (Collision|SetCollisionEnabled _staticmesh "NoCollision"))))))

(fn ConstructionScript)