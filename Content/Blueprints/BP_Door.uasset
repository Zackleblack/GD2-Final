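; BP_Door is a locked door that opens when a BP_FPAbility actor holding a key overlaps its box.
; With a key, the OpenDoor timeline raises the root by lerping from its current location toward a point above it, recomputed each update.
; On finish, the door destroys itself and clears the actor's HasKey flag.
; Without a key, it plays a sound at the Lock's location.
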(event OnComponentBeginOverlap(Box)
  (params (OverlappedComponent :type Primitive%20Component%20Object%20Reference) (OtherActor :type Actor%20Object%20Reference) (OtherComp :type Primitive%20Component%20Object%20Reference) (OtherBodyIndex :type Integer) (bFromSweep :type Boolean) (SweepResult :type Hit%20Result%20Structure%20%28by%20ref%29))
  (bind _defaultsceneroot (Variables|Default|GetDefaultSceneRoot))
  (bind _returnvalue (Transformation|GetWorldLocation _defaultsceneroot))
  (bind _asbp_fpability (Utilities|Casting|CastToBP_FPAbility OtherActor))
  (if (Variables|/Game/Blueprints/TimeTravel/BP_FPAbility.BP_FPAbility_C|GetHasKey? _asbp_fpability)
    (bind _newtrack_0 (Timeline|Open%20Door PlayFromStart)
      (:Update
        (Transformation|SetWorldLocation (Variables|Default|GetDefaultSceneRoot) (Math|Vector|Lerp(Vector) (Math|Vector|MakeVector (.x _returnvalue) (.y _returnvalue) (.z _returnvalue)) (Math|Vector|MakeVector (.x _returnvalue) (.y _returnvalue) (+ (.z _returnvalue) 1e+03)) _newtrack_0) false false))
      (:Finished
        (Actor|DestroyActor)
        (Variables|/Game/Blueprints/TimeTravel/BP_FPAbility.BP_FPAbility_C|SetHasKey? _asbp_fpability false)))
    (else
      (Audio|PlaySoundatLocation 0 (Transformation|GetWorldLocation (Variables|Default|GetLock)) "0, 0, 0" 1.0 1.0 0.0 0 0 0 0))))

(event EventBeginPlay)

(event Collision|EventActorBeginOverlap
  (params (OtherActor :type Actor%20Object%20Reference)))

(event EventTick
  (params (DeltaSeconds :type Float%20%28single-precision%29)))

(fn ConstructionScript)