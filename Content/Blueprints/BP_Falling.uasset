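; BP_Falling is a trigger actor that plays the game's first ending, a fatal fall.
; Box overlap disables input and clears all widgets before checking that the actor is BP_FPAbility.
; For that character it fades to white, plays falling audio and shows the HUD's Ending1 widget, then after a delay cuts to black, removes it and plays a splat.
; BeginPlay caches character, game instance and HUD references, but only the HUD's is used.
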(event OnComponentBeginOverlap(Box)
  (params (OverlappedComponent :type Primitive%20Component%20Object%20Reference) (OtherActor :type Actor%20Object%20Reference) (OtherComp :type Primitive%20Component%20Object%20Reference) (OtherBodyIndex :type Integer) (bFromSweep :type Boolean) (SweepResult :type Hit%20Result%20Structure%20%28by%20ref%29))
  (bind _returnvalue (Game|GetPlayerCameraManager 0))
  (bind _hud_ref (Variables|Default|GetHUD%20Ref))
  (bind _ending_1_reference (Variables|/Game/Blueprints/TimeTravel/BP_FPAbilityHUD.BP_FPAbilityHUD_C|GetEnding%201%20Reference _hud_ref))
  (Input|DisableInput 0)
  (Viewport|RemoveAllWidgets)
  (Utilities|Casting|CastToBP_FPAbility OtherActor)
  (CameraFades|StartCameraFade _returnvalue 0.0 1.0 1.0 "(R=1.000000,G=1.000000,B=1.000000,A=1.000000)" false true)
  (Audio|PlaySound2D "/Game/Audio/FallingSound/FallingSky_Cue.FallingSky_Cue" 0.5 1.0 0.0 0 0)
  (UserInterface|Viewport|AddtoViewport _ending_1_reference 0)
  (Utilities|FlowControl|Delay 16.0)
  (CameraFades|StartCameraFade _returnvalue 1.0 1.0 0.0 "(R=0.000000,G=0.000000,B=0.000000,A=1.000000)" false true)
  (Widget|RemovefromParent _ending_1_reference)
  (Audio|PlaySound2D "/Game/Audio/FallingSound/Splat_Cue.Splat_Cue" 1.0 1.0 0.0 0 0))

(event EventBeginPlay
  (Utilities|FlowControl|Sequence
    (:then_0
      (bind _returnvalue (Actor|GetActorOfClass "/Game/Blueprints/TimeTravel/BP_FPAbility.BP_FPAbility_C"))
      (Variables|Default|SetCharacter%20Ref _returnvalue))
    (:then_1
      (bind _asascend_through_time (Utilities|Casting|CastToAscendThroughTime (Game|GetGameInstance)))
      (Variables|Default|SetGame%20Instance%20REF _asascend_through_time))
    (:then_2
      (bind _returnvalue_2 (Actor|GetActorOfClass "/Game/Blueprints/TimeTravel/BP_FPAbilityHUD.BP_FPAbilityHUD_C"))
      (Variables|Default|SetHUD%20Ref _returnvalue_2))))

(fn ConstructionScript)