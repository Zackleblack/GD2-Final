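; Checkpoint actor that sets the respawn point of a BP_FPAbility actor that touches it.
; Capsule overlap casts the other actor and writes the SpawnLocation component's world position into its RespawnLocation.
; A DoOnce then plays the Checkpoint sound and shows WBP_Checkpoint for a second before removing it and resetting, so feedback cannot stack while the location still saves on every overlap.
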(event OnComponentBeginOverlap(Capsule)
  (params (OverlappedComponent :type Primitive%20Component%20Object%20Reference) (OtherActor :type Actor%20Object%20Reference) (OtherComp :type Primitive%20Component%20Object%20Reference) (OtherBodyIndex :type Integer) (bFromSweep :type Boolean) (SweepResult :type Hit%20Result%20Structure%20%28by%20ref%29))
  (bind _asbp_fpability (Utilities|Casting|CastToBP_FPAbility OtherActor))
  (Variables|/Game/Blueprints/TimeTravel/BP_FPAbility.BP_FPAbility_C|SetRespawnLocation _asbp_fpability (Transformation|GetWorldLocation (Variables|Default|GetSpawnLocation)))
  (Utilities|FlowControl|DoOnce false :!label _label
    (:Completed
      (Audio|PlaySound2D "/Game/Emma/UI/Checkpoint.Checkpoint" 1.0 1.0 0.0 0 0)
      (bind _returnvalue (UserInterface|CreateWidget "/Game/Emma/UI/Dialogue/WBP_Checkpoint.WBP_Checkpoint_C"))
      (UserInterface|Viewport|AddtoViewport _returnvalue 0)
      (Utilities|FlowControl|Delay 1.0)
      (Widget|RemovefromParent _returnvalue)
      (goto _label Reset))))

(event Custom|Save%20Checkpoint%20Start
  (Variables|/Game/Blueprints/TimeTravel/BP_FPAbility.BP_FPAbility_C|SetRespawnLocation (stale OnComponentBeginOverlap(Capsule) _asbp_fpability) (Transformation|GetWorldLocation (Variables|Default|GetSpawnLocation)))
  (Utilities|FlowControl|DoOnce false :!label _label
    (:Completed
      (Audio|PlaySound2D "/Game/Emma/UI/Checkpoint.Checkpoint" 1.0 1.0 0.0 0 0)
      (bind _returnvalue (UserInterface|CreateWidget "/Game/Emma/UI/Dialogue/WBP_Checkpoint.WBP_Checkpoint_C"))
      (UserInterface|Viewport|AddtoViewport _returnvalue 0)
      (Utilities|FlowControl|Delay 1.0)
      (Widget|RemovefromParent _returnvalue)
      (goto _label Reset))))

(event EventBeginPlay)

(event Collision|EventActorBeginOverlap
  (params (OtherActor :type Actor%20Object%20Reference)))

(event EventTick
  (params (DeltaSeconds :type Float%20%28single-precision%29)))

(fn ConstructionScript)