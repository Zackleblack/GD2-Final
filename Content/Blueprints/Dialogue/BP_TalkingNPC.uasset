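; Talking NPC that can optionally roam random nearby navmesh points and converse with the player through its ACDialogue component.
; Sphere overlap plays passive lines automatically or shows an interact prompt; Interact advances dialogue, and leaving resets non-passive dialogue.
; It also handles kid rescue: game-instance flags make Interact trigger a one-time pickup that calls GirlFollowsPlayer and destroys the NPC.
; An already picked-up kid destroys itself on BeginPlay.
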(event OnComponentBeginOverlap(Sphere)
  (params (OverlappedComponent :type Primitive%20Component%20Object%20Reference) (OtherActor :type Actor%20Object%20Reference) (OtherComp :type Primitive%20Component%20Object%20Reference) (OtherBodyIndex :type Integer) (bFromSweep :type Boolean) (SweepResult :type Hit%20Result%20Structure%20%28by%20ref%29))
  (bind _ac_dialogue (Variables|Default|GetAC%20dialogue))
  ;[0 0.4678 0.5333 0.502] NPC Overlap
  (bind _asbp_fpability (Utilities|Casting|CastToBP_FPAbility OtherActor))
  (Variables|Default|SetMain%20Character%20Reference _asbp_fpability)
  (Variables|/Game/Blueprints/Dialogue/AC_Dialogue.AC_Dialogue_C|SetbPlayerInRange? _ac_dialogue true)
  (if (Variables|Default|GetbIsDialoguePassive?)
    (Default|PassiveNextLine _ac_dialogue)
    (else
      (UserInterface|Viewport|AddtoViewport (Variables|/Game/Blueprints/TimeTravel/BP_FPAbilityHUD.BP_FPAbilityHUD_C|GetInteract%20Widget%20Reference (Variables|Default|GetHUD%20Reference)) 0))))

(event OnComponentEndOverlap(Sphere)
  (params (OverlappedComponent :type Primitive%20Component%20Object%20Reference) (OtherActor :type Actor%20Object%20Reference) (OtherComp :type Primitive%20Component%20Object%20Reference) (OtherBodyIndex :type Integer))
  (bind _ac_dialogue (Variables|Default|GetAC%20dialogue))
  ;[0 0.4678 0.5333 0.502] NPC End Overlap
  (Utilities|Casting|CastToBP_FPAbility OtherActor)
  (if (not (Variables|Default|GetbIsDialoguePassive?))
    (Default|ResetDialogue _ac_dialogue)
    (Default|ResetIndex _ac_dialogue)
    (Default|RemoveWidget _ac_dialogue)
    (Widget|RemovefromParent (Variables|/Game/Blueprints/TimeTravel/BP_FPAbilityHUD.BP_FPAbilityHUD_C|GetInteract%20Widget%20Reference (Variables|Default|GetHUD%20Reference)))))

(event Custom|Roam%20Character
  ;[0 0.4678 0.5333 0.502] Comment
  (AI|AIMoveTo self (.RandomLocation (AI|Navigation|GetRandomReachablePointinRadius (Transformation|GetActorLocation) 1.5e+03 0 0)) 0 5.0 false
    (:OnSuccess
      _)
    (:OnFail
      _))
  (Utilities|FlowControl|Delay 1.5)
  (CallFunction|RoamCharacter))

(event Custom|Kid%20Pick%20Up
  (bind _hud_reference (Variables|Default|GetHUD%20Reference))
  (bind _pickup_widget_reference (Variables|/Game/Blueprints/TimeTravel/BP_FPAbilityHUD.BP_FPAbilityHUD_C|GetPickup%20Widget%20Reference _hud_reference))
  (Utilities|FlowControl|DoOnce false
    (:Completed
      (UserInterface|Viewport|AddtoViewport _pickup_widget_reference 0)
      (Development|SetHiddeninGame (Variables|Character|GetMesh) true false)
      (Widget|RemovefromParent _pickup_widget_reference)
      (Default|GirlFollowsPlayer (Variables|Default|GetCharacter%20Reference))
      (Variables|/Game/Blueprints/AscendThroughTime.AscendThroughTime_C|SetbKidPickedUp? (Variables|Default|GetGame%20Instance%20Reference) true)
      (Utilities|FlowControl|Delay 1.0)
      (Actor|DestroyActor))))

(event EventBeginPlay
  ;[0 0.4678 0.5333 0.502] Event begin Play
  (Utilities|FlowControl|Sequence
    (:then_0
      (if (Variables|Default|GetbShouldNPCRoam?)
        (CallFunction|RoamCharacter)))
    (:then_1
      (bind _returnvalue (Actor|GetActorOfClass "/Game/Blueprints/TimeTravel/BP_FPAbilityHUD.BP_FPAbilityHUD_C"))
      (Variables|Default|SetHUD%20Reference _returnvalue))
    (:then_2
      (bind _asascend_through_time (Utilities|Casting|CastToAscendThroughTime (Game|GetGameInstance)))
      (Variables|Default|SetGame%20Instance%20Reference _asascend_through_time))
    (:then_3
      (if (Variables|Default|GetbCanBeRescued?)
        (if (Variables|/Game/Blueprints/AscendThroughTime.AscendThroughTime_C|GetbWentBack? (Variables|Default|GetGame%20Instance%20Reference))
          (Variables|/Game/Blueprints/AscendThroughTime.AscendThroughTime_C|SetbKidFollows? (Variables|Default|GetGame%20Instance%20Reference) true))))
    (:then_4
      (bind _asbp_fpability (Utilities|Casting|CastToBP_FPAbility (Game|GetPlayerCharacter 0)))
      (Variables|Default|SetCharacter%20Reference _asbp_fpability))
    (:then_5
      (if (Variables|Default|GetbIsThisKid?)
        (if (Variables|/Game/Blueprints/AscendThroughTime.AscendThroughTime_C|GetbKidPickedUp? (Variables|Default|GetGame%20Instance%20Reference))
          (Actor|DestroyActor))))))

(event EventInteract
  ;[0 0.4678 0.5333 0.502] NPC Overlap
  (if (not (Variables|Default|GetbIsDialoguePassive?))
    (if (Variables|/Game/Blueprints/AscendThroughTime.AscendThroughTime_C|GetbKidFollows? (Variables|Default|GetGame%20Instance%20Reference))
      (CallFunction|KidPickUp)
      (Widget|RemovefromParent (Variables|/Game/Blueprints/TimeTravel/BP_FPAbilityHUD.BP_FPAbilityHUD_C|GetInteract%20Widget%20Reference (Variables|Default|GetHUD%20Reference)))
      (else
        (Default|NextLineText (Variables|Default|GetAC%20dialogue))
        (Widget|RemovefromParent (Variables|/Game/Blueprints/TimeTravel/BP_FPAbilityHUD.BP_FPAbilityHUD_C|GetInteract%20Widget%20Reference (Variables|Default|GetHUD%20Reference)))))))

(fn ConstructionScript)