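; Dialogue component that steps through DT_Dialogue rows, showing speaker, portrait and text on the ability HUD's dialogue widget with 2D voice playback.
; BeginPlay caches the HUD and starting line; NextLineText advances while the player is in range and dialogue is unfinished.
; A DoOnce gates adding the widget to the viewport.
; Blank-spot indices remove the widget, and a missing row also marks dialogue finished.
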(event Custom|Next%20Line%20Text
  (if (not (Variables|Default|GetbDialogueFinished))
    (if (Variables|Default|GetbPlayerInRange?)
      (if (< (Variables|Default|GetLine%20Index) (Utilities|Array|LastIndex (Variables|Default|GetDialogue)))
        (if (Utilities|Array|ContainsItem (Variables|Default|GetBlank%20Spots) (Variables|Default|GetLine%20Index))
          (Widget|RemovefromParent (Variables|/Game/Blueprints/TimeTravel/BP_FPAbilityHUD.BP_FPAbilityHUD_C|GetDialogue%20Widget%20Reference (Variables|Default|GetHUD%20Reference)))
          (else
            (Utilities|FlowControl|Sequence
              (:then_0
                (Utilities|FlowControl|DoOnce false
                  (:Completed
                    (UserInterface|Viewport|AddtoViewport (Variables|/Game/Blueprints/TimeTravel/BP_FPAbilityHUD.BP_FPAbilityHUD_C|GetDialogue%20Widget%20Reference (Variables|Default|GetHUD%20Reference)) 0))))
              (:then_1
                (bind _outrownames (DataTable|GetDataTableRowNames "/Game/Blueprints/Dialogue/DT_Dialogue.DT_Dialogue"))
                (bind _returnvalue (Utilities|GetDataTableRow "/Game/Blueprints/Dialogue/DT_Dialogue.DT_Dialogue" (Utilities|Array|Get(acopy) _outrownames (Variables|Default|GetLine%20Index)))
                  (:then
                    (CallFunction|DialogueFunction (.characterimage _returnvalue) (.voicedialogue _returnvalue) (.speaker _returnvalue) (.dialogue _returnvalue)))
                  (:RowNotFound
                    (Development|PrintString "Widget Removed")
                    (Widget|RemovefromParent (Variables|/Game/Blueprints/TimeTravel/BP_FPAbilityHUD.BP_FPAbilityHUD_C|GetDialogue%20Widget%20Reference (Variables|Default|GetHUD%20Reference)))
                    (Variables|Default|SetbDialogueFinished true)))))))))))

(event Custom|Reset%20Dialogue
  (Utilities|FlowControl|DoOnce false) ; enters at Reset
)

(event Custom|Add%20Widget
  (UserInterface|Viewport|AddtoViewport (Variables|/Game/Blueprints/TimeTravel/BP_FPAbilityHUD.BP_FPAbilityHUD_C|GetDialogue%20Widget%20Reference (Variables|Default|GetHUD%20Reference)) 0))

(event Custom|Remove%20Widget
  (Widget|RemovefromParent (Variables|/Game/Blueprints/TimeTravel/BP_FPAbilityHUD.BP_FPAbilityHUD_C|GetDialogue%20Widget%20Reference (Variables|Default|GetHUD%20Reference))))

(event Custom|Reset%20Index
  (Variables|Default|SetLine%20Index (Variables|Default|GetLine%20Start)))

(event EventBeginPlay
  (Utilities|FlowControl|Sequence
    (:then_0
      (bind _returnvalue (Actor|GetActorOfClass "/Game/Blueprints/TimeTravel/BP_FPAbilityHUD.BP_FPAbilityHUD_C"))
      (bind _output_get (Variables|Default|SetHUD%20Reference _returnvalue))
      (Variables|Default|SetDialogue%20Widget%20Reference (Variables|/Game/Blueprints/TimeTravel/BP_FPAbilityHUD.BP_FPAbilityHUD_C|GetDialogue%20Widget%20Reference _output_get)))
    (:then_1
      (Variables|Default|SetLine%20Index (Variables|Default|GetLine%20Start)))))

(fn DialogueFunction
  (params (Texture :type Texture%202D%20Object%20Reference) (Sound :type Sound%20Base%20Object%20Reference) (Value :type E_Speaker%20Enum :default "NewEnumerator1") (InText :type Text))
  (Development|PrintString "Dialogue Function hit")
  (bind _result (Math|Integer|IncrementInt (Variables|Default|GetLine%20Index))
    (:%20%20
      (Development|PrintString (Utilities|String|ToString(Integer) _result))
      (Audio|PlaySound2D Sound 1.0 1.0 0.0 0 0)
      (Appearance|SetBrushfromTexture (Variables|/Game/Blueprints/Dialogue/WBP_Dialogue.WBP_Dialogue_C|GetCharacterIMG (Variables|/Game/Blueprints/TimeTravel/BP_FPAbilityHUD.BP_FPAbilityHUD_C|GetDialogue%20Widget%20Reference (Variables|Default|GetHUD%20Reference))) Texture false)
      (Rendering|Components|TextRender|SetText (Variables|/Game/Blueprints/Dialogue/WBP_Dialogue.WBP_Dialogue_C|GetDialogueText (Variables|/Game/Blueprints/TimeTravel/BP_FPAbilityHUD.BP_FPAbilityHUD_C|GetDialogue%20Widget%20Reference (Variables|Default|GetHUD%20Reference))) InText)
      (Rendering|Components|TextRender|SetText (Variables|/Game/Blueprints/Dialogue/WBP_Dialogue.WBP_Dialogue_C|GetNameText (Variables|/Game/Blueprints/TimeTravel/BP_FPAbilityHUD.BP_FPAbilityHUD_C|GetDialogue%20Widget%20Reference (Variables|Default|GetHUD%20Reference))) (|GenerictoText Value))
      (Development|PrintString "Dialogue Function Finished")
      (Variables|Default|SetDialogue%20Widget%20Reference (Variables|Default|GetDialogue%20Widget%20Reference))
      (return))))