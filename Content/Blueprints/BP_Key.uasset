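; BP_Key is a key pickup that spins and bobs using two timelines started on BeginPlay.
; Entering its ReachSphere aims the player's right-hand IK in ABP_Manny at the key's location, captured once on overlap, and leaving switches the IK off.
; Overlapping Sphere clears the IK, sets HasKey on BP_FPAbility and destroys the key.
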(event OnComponentBeginOverlap(ReachSphere)
  (params (OverlappedComponent :type Primitive%20Component%20Object%20Reference) (OtherActor :type Actor%20Object%20Reference) (OtherComp :type Primitive%20Component%20Object%20Reference) (OtherBodyIndex :type Integer) (bFromSweep :type Boolean) (SweepResult :type Hit%20Result%20Structure%20%28by%20ref%29))
  (bind _asbp_fpability (Utilities|Casting|CastToBP_FPAbility OtherActor))
  (bind _asabp_manny (Utilities|Casting|CastToABP_Manny (Components|SkeletalMesh|GetAnimInstance (Variables|/Script/Engine.Character|GetMesh _asbp_fpability))))
  (Variables|/Game/CR/Demo/Animations/ABP_Manny.ABP_Manny_C|SetRightHandIKTarget _asabp_manny (Transformation|GetWorldLocation (Variables|Default|GetKey)))
  (Variables|/Game/CR/Demo/Animations/ABP_Manny.ABP_Manny_C|SetRightHandIKAlpha _asabp_manny 1.0))

(event OnComponentEndOverlap(ReachSphere)
  (params (OverlappedComponent :type Primitive%20Component%20Object%20Reference) (OtherActor :type Actor%20Object%20Reference) (OtherComp :type Primitive%20Component%20Object%20Reference) (OtherBodyIndex :type Integer))
  (bind _asbp_fpability (Utilities|Casting|CastToBP_FPAbility OtherActor))
  (bind _asabp_manny (Utilities|Casting|CastToABP_Manny (Components|SkeletalMesh|GetAnimInstance (Variables|/Script/Engine.Character|GetMesh _asbp_fpability))))
  (Variables|/Game/CR/Demo/Animations/ABP_Manny.ABP_Manny_C|SetRightHandIKAlpha _asabp_manny 0.0))

(event OnComponentBeginOverlap(Sphere)
  (params (OverlappedComponent :type Primitive%20Component%20Object%20Reference) (OtherActor :type Actor%20Object%20Reference) (OtherComp :type Primitive%20Component%20Object%20Reference) (OtherBodyIndex :type Integer) (bFromSweep :type Boolean) (SweepResult :type Hit%20Result%20Structure%20%28by%20ref%29))
  (bind _asbp_fpability (Utilities|Casting|CastToBP_FPAbility OtherActor))
  (bind _asabp_manny (Utilities|Casting|CastToABP_Manny (Components|SkeletalMesh|GetAnimInstance (Variables|/Script/Engine.Character|GetMesh _asbp_fpability))))
  (Variables|/Game/CR/Demo/Animations/ABP_Manny.ABP_Manny_C|SetRightHandIKAlpha _asabp_manny 0.0)
  (Variables|/Game/Blueprints/TimeTravel/BP_FPAbility.BP_FPAbility_C|SetHasKey? _asbp_fpability true)
  (Actor|DestroyActor))

(event EventBeginPlay
  (bind _key (Variables|Default|GetKey))
  (bind _returnvalue (Transformation|GetRelativeTransform _key))
  (Utilities|FlowControl|Sequence
    (:then_0
      (bind _loop (Timeline|Timeline Play)
        (:Update
          (Transformation|SetRelativeRotation _key (Math|Rotator|MakeRotator 0.0 (Math|Float|Lerp 0.0 3.6e+02 _loop) 0.0) false false))))
    (:then_1
      (bind _loop_2 (Timeline|Timeline_0 Play)
        (:Update
          (Transformation|SetRelativeLocation _key (Math|Vector|MakeVector (.x (.location _returnvalue)) (.y (.location _returnvalue)) (Math|Float|Lerp 0.0 3e+01 _loop_2)) false false))))))

(fn ConstructionScript)