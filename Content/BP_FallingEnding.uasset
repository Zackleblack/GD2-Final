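; Trigger volume actor that plays the falling ending when BP_FPAbility enters its box.
; Any overlap clears all widgets, then for that player it plays music and wind, fades to white and shows the Ending1 widget from BP_FPAbilityHUD.
; After a timed delay it removes the widget, plays a falling sound and cuts to held black.
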(event OnComponentBeginOverlap(Box)
  (params (OverlappedComponent :type Primitive%20Component%20Object%20Reference) (OtherActor :type Actor%20Object%20Reference) (OtherComp :type Primitive%20Component%20Object%20Reference) (OtherBodyIndex :type Integer) (bFromSweep :type Boolean) (SweepResult :type Hit%20Result%20Structure%20%28by%20ref%29))
  (bind _returnvalue (Game|GetPlayerController 0))
  (bind _hud_ref (Variables|Default|GetHUD%20Ref))
  (bind _ending_1_ref (Variables|/Game/Blueprints/TimeTravel/BP_FPAbilityHUD.BP_FPAbilityHUD_C|GetEnding%201%20Ref _hud_ref))
  (bind _playercameramanager (Variables|/Script/Engine.PlayerController|GetPlayerCameraManager _returnvalue))
  (Viewport|RemoveAllWidgets)
  (Utilities|Casting|CastToBP_FPAbility OtherActor)
  (Audio|PlaySound2D "/Game/Emma/Audio/UI/sonican-enchanted-fantasy-classical-music-516862.sonican-enchanted-fantasy-classical-music-516862" (Variables|Default|GetVolume%20Multiplier) 1.0 0.0 0 0)
  (CameraFades|StartCameraFade _playercameramanager 0.0 1.0 1.0 "(R=1.000000,G=1.000000,B=1.000000,A=1.000000)" false true)
  (Audio|PlaySound2D "/Game/Audio/dragon-studio-wind-blowing-sfx-07-423677.dragon-studio-wind-blowing-sfx-07-423677" 0.3 1.0 0.0 0 0)
  (UserInterface|Viewport|AddtoViewport _ending_1_ref 0)
  (Utilities|FlowControl|Delay 16.0)
  (Widget|RemovefromParent _ending_1_ref)
  (Audio|PlaySound2D "/Game/Audio/universfield-falling-game-character-352287.universfield-falling-game-character-352287" 1.0 1.0 0.0 0 0)
  (Variables|Default|SetVolume%20Multiplier 0.0)
  (CameraFades|StartCameraFade _playercameramanager 1.0 1.0 0.0 "(R=0.000000,G=0.000000,B=0.000000,A=1.000000)" false true)
  (Utilities|FlowControl|Delay 2.0))

(event EventBeginPlay
  (bind _returnvalue (Actor|GetActorOfClass "/Game/Blueprints/TimeTravel/BP_FPAbilityHUD.BP_FPAbilityHUD_C"))
  (Variables|Default|SetHUD%20Ref _returnvalue))

(fn ConstructionScript)